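; BP_Player is the player Blueprint, holding a test hook for ending the game when its timer runs out.
; BeginPlay casts the game instance to MyGameInstance and caches the reference.
; EndTimerEvent, marked as testing, reads TotalTime from that instance and quits the game at zero or below, otherwise printing a debug message.
; Nothing in this Blueprint calls that event, and Tick and overlap are unimplemented.
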(event EventBeginPlay
  (bind _asmy_game_instance (Utilities|Casting|CastToMyGameInstance (Game|GetGameInstance)))
  (Variables|Default|SetGameInstaceRef _asmy_game_instance))

(event Collision|EventActorBeginOverlap
  (params (OtherActor :type Actor%20Object%20Reference)))

(event EventTick
  (params (DeltaSeconds :type Float%20%28single-precision%29)))

(event EventEndTimerEvent
  ;[1 0 0] TESTING -- Game Timer Event
  (if (<= (Variables|/Script/CarCentric.MyGameInstance|GettotalTime (Variables|Default|GetGameInstaceRef)) 0)
    (Game|QuitGame (Game|GetPlayerController 0) "Quit" false)
    (else
      (Development|PrintString "NOT DONE YET"))))

(fn ConstructionScript)